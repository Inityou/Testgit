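; BP_door_End is a key-gated door, likely the level's end door, with a timeline that raises Door2 vertically.
; Box overlap checks Block1 and Block2, printing Russian hints about missing keys while either is set.
; When both are clear, a Popi entering triggers opening and any actor leaving triggers closing, each after a short delay.
; Neither flag is changed within this Blueprint.
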(event OnComponentBeginOverlap(Box)
  (params (OverlappedComponent :type Primitive%20Component%20Object%20Reference) (OtherActor :type Actor%20Object%20Reference) (OtherComp :type Primitive%20Component%20Object%20Reference) (OtherBodyIndex :type Integer) (bFromSweep :type Boolean) (SweepResult :type Hit%20Result%20Structure%20%28by%20ref%29))
  (if (Variables|Default|GetBlock_1)
    (Development|PrintString "Найди первый и второй ключ")
    (elif (Variables|Default|GetBlock_2)
      (Development|PrintString "Найди втрой ключ")
      (else
        (Utilities|Casting|CastToPopi OtherActor)
        (Utilities|FlowControl|Delay 0.1)
        (CallFunction|OpenDoor)))))

(event OnComponentEndOverlap(Box)
  (params (OverlappedComponent :type Primitive%20Component%20Object%20Reference) (OtherActor :type Actor%20Object%20Reference) (OtherComp :type Primitive%20Component%20Object%20Reference) (OtherBodyIndex :type Integer))
  (if (not (Variables|Default|GetBlock_1))
    (if (not (Variables|Default|GetBlock_2))
      (Utilities|FlowControl|Delay 0.2)
      (CallFunction|CloseDoor))))

(event Custom|Open_door
  (Components|Timeline|PlayfromStart (Variables|Default|Getdoor)))

(event Custom|Close_door
  (Utilities|String|Reverse (Variables|Default|Getdoor)))

(fn ConstructionScript)