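; Door Blueprint that opens when something enters its trigger box and closes when it leaves, unless a BLOCK flag locks it.
; Box overlap events wait briefly before calling open or close, while a blocked door only prints that a key is needed on entry.
; A Door timeline, played forward or in reverse, interpolates the rotation of Door2 to swing it through 90 degrees.
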(event OnComponentBeginOverlap(Box)
  (params (OverlappedComponent :type Primitive%20Component%20Object%20Reference) (OtherActor :type Actor%20Object%20Reference) (OtherComp :type Primitive%20Component%20Object%20Reference) (OtherBodyIndex :type Integer) (bFromSweep :type Boolean) (SweepResult :type Hit%20Result%20Structure%20%28by%20ref%29))
  (if (Variables|Default|GetBLOCK)
    (Development|PrintString "Need a key")
    (else
      (Utilities|FlowControl|Delay 0.1)
      (CallFunction|OpenDoor))))

(event OnComponentEndOverlap(Box)
  (params (OverlappedComponent :type Primitive%20Component%20Object%20Reference) (OtherActor :type Actor%20Object%20Reference) (OtherComp :type Primitive%20Component%20Object%20Reference) (OtherBodyIndex :type Integer))
  (if (not (Variables|Default|GetBLOCK))
    (Utilities|FlowControl|Delay 0.1)
    (CallFunction|CloseDoor)))

(event Custom|Open_door
  (bind _door (Timeline|door PlayFromStart)
    (:Update
      (Transformation|SetRelativeRotation (Variables|Default|Getdoor2) (Math|Rotator|Lerp(Rotator) "0, 0, 0" "0,90.000000, 0" _door) false false))))

(event Custom|Close_door
  (bind _door (Timeline|door ReverseFromEnd)
    (:Update
      (Transformation|SetRelativeRotation (Variables|Default|Getdoor2) (Math|Rotator|Lerp(Rotator) "0, 0, 0" "0,90.000000, 0" _door) false false))))

(fn ConstructionScript)