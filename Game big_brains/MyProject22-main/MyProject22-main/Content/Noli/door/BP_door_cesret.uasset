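; Interactable door Blueprint that swings a mesh component, Floor2, open and then closes it automatically.
; A timeline's Door track drives lerps of Floor2's relative rotation and location, producing a quarter turn combined with a sideways shift, teleported without sweep.
; Interact plays the timeline through Start, waits a fixed one-second delay, then calls End to reverse it from the end.
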(event Custom|Start
  (bind _floor2 (Variables|Default|Getfloor2))
  (bind _door (Timeline|Time Play)
    (:Update
      (Transformation|SetRelativeRotation _floor2 (Math|Rotator|Lerp(Rotator) "0,-180.000000,270.000000" "0.000000,-270.000000,270.000000" _door) false false)
      (Transformation|SetRelativeLocation _floor2 (Math|Vector|Lerp(Vector) "0.000000, 0,68.000000" "-50.000000,-65.000000,68.000000" _door) false true))))

(event Custom|end
  (bind _floor2 (Variables|Default|Getfloor2))
  (bind _door (Timeline|Time ReverseFromEnd)
    (:Update
      (Transformation|SetRelativeRotation _floor2 (Math|Rotator|Lerp(Rotator) "0,-180.000000,270.000000" "0.000000,-270.000000,270.000000" _door) false false)
      (Transformation|SetRelativeLocation _floor2 (Math|Vector|Lerp(Vector) "0.000000, 0,68.000000" "-50.000000,-65.000000,68.000000" _door) false true))))

(event EventInteract
  (CallFunction|Start)
  (Utilities|FlowControl|Delay 1.0)
  (CallFunction|End))

(fn ConstructionScript)