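; Sliding door Blueprint from the Noli puzzle folder that opens when something overlaps its trigger box and can be locked.
; The Box overlap events check BLOCK2: while set, entering prints a key-needed message, otherwise entering and leaving call open and close after a short delay.
; The Door timeline drives a relative-location lerp on Door2, playing from start to open and reversing from end to close.
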(event OnComponentBeginOverlap(Box)
  (params (OverlappedComponent :type Primitive%20Component%20Object%20Reference) (OtherActor :type Actor%20Object%20Reference) (OtherComp :type Primitive%20Component%20Object%20Reference) (OtherBodyIndex :type Integer) (bFromSweep :type Boolean) (SweepResult :type Hit%20Result%20Structure%20%28by%20ref%29))
  (if (Variables|Default|GetBLOCK2)
    (Development|PrintString "Need a key")
    (else
      (Utilities|FlowControl|Delay 0.1)
      (CallFunction|OpenDoor))))

(event OnComponentEndOverlap(Box)
  (params (OverlappedComponent :type Primitive%20Component%20Object%20Reference) (OtherActor :type Actor%20Object%20Reference) (OtherComp :type Primitive%20Component%20Object%20Reference) (OtherBodyIndex :type Integer))
  (if (not (Variables|Default|GetBLOCK2))
    (Utilities|FlowControl|Delay 0.1)
    (CallFunction|CloseDoor)))

(event Custom|Open_door
  (bind _door (Timeline|door PlayFromStart)
    (:Update
      (Transformation|SetRelativeLocation (Variables|Default|Getdoor2) (Math|Vector|Lerp(Vector) "0,-176.000000, 0" "0,176.000000,0.000000" _door) false false))))

(event Custom|Close_door
  (bind _door (Timeline|door ReverseFromEnd)
    (:Update
      (Transformation|SetRelativeLocation (Variables|Default|Getdoor2) (Math|Vector|Lerp(Vector) "0,-176.000000, 0" "0,176.000000,0.000000" _door) false false))))

(fn ConstructionScript)